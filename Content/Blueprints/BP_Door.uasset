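; Door Blueprint that the player opens and closes with the Interact input while standing in its box trigger and holding a key.
; Overlap with the ThirdPersonCharacter caches the character, toggles input on the door and opens or closes a Gate.
; Interact checks the character's HasKey, printing a message without it, then passes through the Gate to a FlipFlop.
; The FlipFlop plays or reverses a timeline that lerps the door's yaw between closed and open angles.
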(event `InputAction|Interact`
  (params (Key :type "Key Structure"))
  ;[1 1 1] Open door if has key
  (:`Pressed`
    (if (`/Game/ThirdPersonBP/Blueprints/ThirdPersonCharacter.HasKey` (stale `self.BoxCollision.OnComponentBeginOverlap` _asthird_person_character))
      (`/Engine/EditorBlueprintResources/StandardMacros.Gate` true :!label _label
        (:`Exit`
          ;[1 1 1] Open\Close Door Animation
          (`/Engine/EditorBlueprintResources/StandardMacros.FlipFlop`
            (:`A`
              (bind (_direction _door_track) (`Timeline|Open\\Close Door` :!label _label_2)
                (:`Update`
                  (`SceneComponent.K2_SetRelativeRotation` (`self.Door`) (`KismetMathLibrary.MakeRotator` 0.0 0.0 (`KismetMathLibrary.Lerp` (`self.DoorClosedAngle`) (`self.DoorOpenAngle`) _door_track)) false false))))
            (:`B`
              (goto _label_2 :!via `Reverse`)))))
      (else
        (`KismetSystemLibrary.PrintString` "You need a key to open the door" true true (struct :`R` 1.0 :`B` 0.017682 :`A` 1.0) 3.0)))))

(event `self.BoxCollision.OnComponentBeginOverlap`
  (params (OverlappedComponent :type "PrimitiveComponent Object Reference") (OtherActor :type "Actor Object Reference") (OtherComp :type "PrimitiveComponent Object Reference") (OtherBodyIndex :type Integer) (bFromSweep :type Boolean) (SweepResult :type "HitResult Structure (by ref)"))
  ;[1 1 1] Open door if has key
  (bind _asthird_person_character (cast `/Game/ThirdPersonBP/Blueprints/ThirdPersonCharacter` OtherActor))
  (`self.EnableInput` (`GameplayStatics.GetPlayerController` 0))
  (goto _label :!via `Open`))

(event `self.BoxCollision.OnComponentEndOverlap`
  (params (OverlappedComponent :type "PrimitiveComponent Object Reference") (OtherActor :type "Actor Object Reference") (OtherComp :type "PrimitiveComponent Object Reference") (OtherBodyIndex :type Integer))
  ;[1 1 1] Open door if has key
  (cast `/Game/ThirdPersonBP/Blueprints/ThirdPersonCharacter` OtherActor)
  (`self.DisableInput` (`GameplayStatics.GetPlayerController` 0))
  (goto _label :!via `Close`))

(fn `UserConstructionScript`)