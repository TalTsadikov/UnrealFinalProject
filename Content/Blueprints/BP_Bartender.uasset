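; BP_Bartender is a quest-giver for the sumo match fetch quest, sending the player after salt, water and paper of strength.
; A Box overlap toggles input on the actor, so Interact works only nearby.
; Interact reads QuestState from the ThirdPersonCharacter to pick the text for a WB_QuestWindow, created in the first stage and reused later, then switches input to UI-only.
; An already accepted first quest only prints a reminder.
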(event `self.ReceiveBeginPlay`
  (bind _asthird_person_character (cast `/Game/ThirdPersonBP/Blueprints/ThirdPersonCharacter` (`GameplayStatics.GetPlayerPawn` 0)))
  (set `self.Player` _asthird_person_character))

(event `self.Box.OnComponentBeginOverlap`
  (params (OverlappedComponent :type "PrimitiveComponent Object Reference") (OtherActor :type "Actor Object Reference") (OtherComp :type "PrimitiveComponent Object Reference") (OtherBodyIndex :type Integer) (bFromSweep :type Boolean) (SweepResult :type "HitResult Structure (by ref)"))
  (if (== OtherActor (`GameplayStatics.GetPlayerPawn` 0))
    (`self.EnableInput` (`GameplayStatics.GetPlayerController` 0))))

(event `self.Box.OnComponentEndOverlap`
  (params (OverlappedComponent :type "PrimitiveComponent Object Reference") (OtherActor :type "Actor Object Reference") (OtherComp :type "PrimitiveComponent Object Reference") (OtherBodyIndex :type Integer))
  (if (== OtherActor (`GameplayStatics.GetPlayerPawn` 0))
    (`self.DisableInput` (`GameplayStatics.GetPlayerController` 0))))

(event `InputAction|Interact`
  (params (Key :type "Key Structure"))
  (:`Pressed`
    (switch `int` (`/Game/ThirdPersonBP/Blueprints/ThirdPersonCharacter.QuestState` (`self.Player`))
      (:`0`
        (if (`/Game/ThirdPersonBP/Blueprints/ThirdPersonCharacter.HasAcceptedQuest` (`self.Player`))
          (`KismetSystemLibrary.PrintString` "I already told you what to do.... go already" true true (struct :`R` 1.0 :`G` 0.006121 :`A` 1.0))
          (else
            (`/Engine/EditorBlueprintResources/StandardMacros.IsValid` (`self.Quest Window`)
              (:`Is Valid`
                _)
              (:`Is Not Valid`
                (bind _returnvalue (`|CreateWidget` "/Game/Widgets/WB_QuestWindow.WB_QuestWindow_C" null "The Great Sumo Match" "Your mission, should you choose to accept it, is to recover the salt bag for the great sumo match. Without it the sumo wrestlers can't start their match."))
                (bind _output_get (set `self.Quest Window` _returnvalue))))
            (`UserWidget.AddToViewport` _output_get 0 :!label _label)
            (`WidgetBlueprintLibrary.SetInputMode_UIOnlyEx` (`GameplayStatics.GetPlayerController` 0) _output_get))))
      (:`1`
        (set `/Game/Widgets/WB_QuestWindow.BodyText` "Ok, now that you have the salt bag, the sumo wrestlers still need their chikara mizu (Water of strength). Without it the sumo wrestlers can't start their match." (`self.Quest Window`))
        (goto _label))
      (:`2`
        (set `/Game/Widgets/WB_QuestWindow.BodyText` "Ok, now that you have the chikara mizu, the sumo wrestlers still need their chikara gami (Paper of strength). Without it the sumo wrestlers can't start their match." (`self.Quest Window`))
        (goto _label)))))

(fn `UserConstructionScript`)