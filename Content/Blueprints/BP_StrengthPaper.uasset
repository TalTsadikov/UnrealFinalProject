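; Interactable pickup actor for the "chikara gami" strength paper quest item.
; Overlapping its box enables player input and opens a gate, so Interact only works while something is inside; leaving reverses both.
; On interact, if the overlapping ThirdPersonCharacter has collected the Water of Strength, it sets QuestState to 3 and hides the paper, otherwise prints a refusal message.
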(event `InputAction|Interact`
  (params (Key :type "Key Structure"))
  (:`Pressed`
    (`/Engine/EditorBlueprintResources/StandardMacros.Gate` true :!label _label
      (:`Exit`
        (bind _asthird_person_character (cast `/Game/ThirdPersonBP/Blueprints/ThirdPersonCharacter` (stale `self.BoxCollision.OnComponentBeginOverlap` OtherActor) :!pure true))
        (if (`/Game/ThirdPersonBP/Blueprints/ThirdPersonCharacter.HasCollectedWaterOfStrength` _asthird_person_character)
          (set `/Game/ThirdPersonBP/Blueprints/ThirdPersonCharacter.QuestState` 3 _asthird_person_character)
          (`KismetSystemLibrary.PrintString` "Collected chikara gami" true true (struct :`R` 0.013873 :`G` 1.0 :`A` 1.0) 3.0)
          (`self.SetActorHiddenInGame` true)
          (else
            (`KismetSystemLibrary.PrintString` "Not yet young one" true true (struct :`R` 1.0 :`G` 0.055564 :`A` 1.0))))))))

(event `self.BoxCollision.OnComponentBeginOverlap`
  (params (OverlappedComponent :type "PrimitiveComponent Object Reference") (OtherActor :type "Actor Object Reference") (OtherComp :type "PrimitiveComponent Object Reference") (OtherBodyIndex :type Integer) (bFromSweep :type Boolean) (SweepResult :type "HitResult Structure (by ref)"))
  (`self.EnableInput` (`GameplayStatics.GetPlayerController` 0))
  (goto _label :!via `Open`))

(event `self.BoxCollision.OnComponentEndOverlap`
  (params (OverlappedComponent :type "PrimitiveComponent Object Reference") (OtherActor :type "Actor Object Reference") (OtherComp :type "PrimitiveComponent Object Reference") (OtherBodyIndex :type Integer))
  (`self.DisableInput` (`GameplayStatics.GetPlayerController` 0))
  (goto _label :!via `Close`))

(fn `UserConstructionScript`)